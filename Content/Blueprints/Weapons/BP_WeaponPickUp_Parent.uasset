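; Parent Blueprint for weapon pickups that hand the player a new weapon and can show item-specific quest text.
; Interact spawns the Weapon class far below the origin, passes it to the player's LinkNewWeapon, then hides the mesh, disables its collision and clears the interact prompt.
; PickUpItem calls InitialiseQuest, which creates a quest from custom texts through the player's quest system and fades its popup after a delay.
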(event `/Game/StudentWork/BI_Interaction.Interact`
  (bind _staticmesh (`self.StaticMesh`))
  ;[1 1 1] When the Player Collides, update their existing weapon with the new one, then destroy this pick up
  (bind _asbp_player_character (cast `/Game/StudentWork/Blueprints/BP_PlayerCharacter` (`GameplayStatics.GetPlayerCharacter` 0)))
  (bind _returnvalue (`|SpawnActorFromClass` (`self.Weapon`) (`KismetMathLibrary.MakeTransform` (0.0 0.0 -5000.0)) "Undefined" "MultiplyWithRoot" null null))
  (bind _asbp_base_weapon_parent (cast `/Game/Blueprints/Weapons/BP_BaseWeapon_Parent` _returnvalue))
  (`/Game/StudentWork/Blueprints/BP_PlayerCharacter.LinkNewWeapon` _asbp_player_character _asbp_base_weapon_parent)
  (`SceneComponent.SetVisibility` _staticmesh false true)
  (`PrimitiveComponent.SetCollisionEnabled` _staticmesh "NoCollision")
  (`/Game/StudentWork/UI/WBP_InteractPrompt.HideInteractPrompt` (`/Game/StudentWork/Blueprints/BP_PlayerCharacter.InteractPromptRef` _asbp_player_character)))

(event `InitialiseQuest`
  ;[1 1 1] Sets up quest system to display specific quest information from this item instance
  (`self.PlayerCharacterRef`
    (:`then`
      _)
    (:`else`
      (bind _asbp_player_character (cast `/Game/StudentWork/Blueprints/BP_PlayerCharacter` (`GameplayStatics.GetPlayerCharacter` 0)))))
  (bind _ac_questsystem (`/Game/StudentWork/Blueprints/BP_PlayerCharacter.AC_QuestSystem` _asbp_player_character))
  (`/Game/StudentWork/Blueprints/Quests/AC_QuestSystem.CreateQuest` _ac_questsystem (`self.CustomQuestTypeText`) (`self.CustomQuestText`) (`self.CustomTipText`))
  (`KismetSystemLibrary.Delay` 4.0)
  (`/Game/StudentWork/UI/WBP_QuestPopup.FadeOut` (`/Game/StudentWork/Blueprints/Quests/AC_QuestSystem.QuestPopupWidgetRef` _ac_questsystem)))

(fn `PickUpItem`
  (returns (Item :type String))
  (`self.InitialiseQuest`)
  (return ""))

(fn `UserConstructionScript`
  (`parent.UserConstructionScript`))