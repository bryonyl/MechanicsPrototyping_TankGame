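; BP_Minion_FollowPlayer is a minion that follows the player and shoots at its target.
; Its Move event uses AI MoveTo to approach the player character, stopping within a set acceptance radius.
; Its Attack event spawns a small fast projectile at the fire point, rotated to face the target, when that target is valid.
; The construction script only calls the parent, and the graph relies on references it does not set itself.
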(event `self.Move`
  ;[1 1 1] Minion always follows behind player
  (`/Engine/EditorBlueprintResources/StandardMacros.IsValid` (`self.PlayerCharacterRef`)
    (:`Is Valid`
      (`|AIMoveTo` self (0.0 0.0 0.0) (`self.PlayerCharacterRef`) 150.0))))

(event `self.Attack`
  (bind _target (`self.Target`))
  (bind _returnvalue (`SceneComponent.K2_GetComponentLocation` (`self.FirePoint`)))
  (`/Engine/EditorBlueprintResources/StandardMacros.IsValid` _target
    (:`Is Valid`
      (`|SpawnActorFromClass` "/Game/StudentWork/Blueprints/Weapons/BP_SmallFastProjectile.BP_SmallFastProjectile_C" (`KismetMathLibrary.MakeTransform` _returnvalue (`KismetMathLibrary.FindLookAtRotation` _returnvalue (`self.K2_GetActorLocation` _target))) "Undefined" "MultiplyWithRoot" null null))))

(fn `UserConstructionScript`
  (`parent.UserConstructionScript`))