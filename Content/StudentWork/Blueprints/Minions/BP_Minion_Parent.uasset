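; Parent Blueprint for tank-style minions that target actors tagged "Enemy", with empty Move and Attack events.
; Sphere sensor overlaps start looping target-check timers, plus movement and attack timers for enemies or the player.
; Tick snaps the turret toward the target and smoothly turns the hull along velocity.
; Damage updates a player-proximity health bar, flashes an overlay material through a timeline and, at zero health, destroys the minion with a Niagara explosion.
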(event `StartTargetCheckTimer`
  ;[0.1063 0.2664 1] Enemy detection
  ;;[1 1 1] Determines whether the overlapping actor is an enemy (so, a target) or not
  (bind _returnvalue (`KismetSystemLibrary.K2_SetTimerDelegate` (delegate `DetermineTarget`) (`self.TargetCheckTime`) true))
  (set `self.TargetCheckTimer` _returnvalue))

(event `self.SphereSensor.OnComponentBeginOverlap`
  (params (OverlappedComponent :type "PrimitiveComponent Object Reference") (OtherActor :type "Actor Object Reference") (OtherComp :type "PrimitiveComponent Object Reference") (OtherBodyIndex :type Integer) (bFromSweep :type Boolean) (SweepResult :type "HitResult Structure (by ref)"))
  ;[0.1063 0.2664 1] Enemy detection
  ;;[1 1 1] Enemy parent reference and player reference are created. Enemy and player are detected, movement and attack timers start
  (set `self.bMinionUnlocked` true)
  (if (`self.bMinionUnlocked`)
    (`self.StartTargetCheckTimer`)
    (bind _asbp_enemy_parent (cast `/Game/StudentWork/Blueprints/EnemiesAndTraps/BP_Enemy_Parent` OtherActor)
      (:`then`
        (`KismetSystemLibrary.PrintString` "MINION FOUND ENEMY")
        (set `self.EnemyParentRef` _asbp_enemy_parent)
        (set `self.bEnemyDetected` true))
      (:`CastFailed`
        (bind _asbp_player_character (cast `/Game/StudentWork/Blueprints/BP_PlayerCharacter` OtherActor))
        (set `self.PlayerCharacterRef` _asbp_player_character)))
    (`self.StartMovementTimer`)
    (`self.StartAttackTimer`)))

(event `DetermineTarget`
  ;[0.1063 0.2664 1] Enemy detection
  ;;[1 1 1] Determines whether the overlapping actor is an enemy (so, a target) or not
  (for _array_element (`self.GetOverlappingActors` null)
    (if (`self.ActorHasTag` _array_element "Enemy")
      (`KismetSystemLibrary.PrintString` "Detected enemy")
      (set `self.Target` _array_element)
      (break)
      (else
        (`KismetSystemLibrary.PrintString` "Not detected enemy")
        (set `self.Target` (`self.BlankReference`))))))

(event `self.SphereSensor.OnComponentEndOverlap`
  (params (OverlappedComponent :type "PrimitiveComponent Object Reference") (OtherActor :type "Actor Object Reference") (OtherComp :type "PrimitiveComponent Object Reference") (OtherBodyIndex :type Integer))
  ;[0.1063 0.2664 1] Enemy detection
  ;;[1 1 1] Enemy is no longer detected
  (bind _asbp_enemy_parent (cast `/Game/StudentWork/Blueprints/EnemiesAndTraps/BP_Enemy_Parent` OtherActor)
    (:`then`
      (set `self.EnemyParentRef` _asbp_enemy_parent)
      (set `self.bEnemyDetected` false))
    (:`CastFailed`
      (bind _asbp_player_character (cast `/Game/StudentWork/Blueprints/BP_PlayerCharacter` OtherActor))
      (set `self.PlayerCharacterRef` _asbp_player_character))))

(event `StartMovementTimer`
  ;[1 0.05092 0.03103] Minion actions
  ;;[1 1 1] Minion moves
  (bind _returnvalue (`KismetSystemLibrary.K2_SetTimerDelegate` (delegate `Move`) (`self.MovementUpdateTime`) true))
  (set `self.MovementTimer` _returnvalue))

(event `StartAttackTimer`
  ;[1 0.05092 0.03103] Minion actions
  ;;[1 1 1] Minion attacks
  (bind _returnvalue (`KismetSystemLibrary.K2_SetTimerDelegate` (delegate `Attack`) (`self.AttackSpeed`) true))
  (set `self.AttackTimer` _returnvalue))

(event `ChangeMinionColourToRed`
  ;[1 0.05092 0.03103] Minion actions
  ;;[1 1 1] Minion turns red when damaged for a short period of time
  (`/Engine/EditorBlueprintResources/StandardMacros.DoOnce` false :!label _label
    (:`Completed`
      (bind (_direction _flash) (`Timeline|Flash` :!via `PlayFromStart`)
        (:`Update`
          (`MaterialInstanceDynamic.SetScalarParameterValue` (`self.DamageOverlayMat`) "FlashLevel" _flash))
        (:`Finished`
          (goto _label :!via `Reset`))))))

(event `Move`
  ;[1 0.05092 0.03103] Minion actions
  ;;[1 1 1] Minion moves
)

(event `Attack`
  ;[1 0.05092 0.03103] Minion actions
  ;;[1 1 1] Minion attacks
)

(event `MinionDies`
  ;[1 0.05092 0.03103] Minion actions
  ;;[1 1 1] Minion dies
  (set `self.bMinionDead` true)
  (`self.K2_DestroyActor`)
  (`NiagaraFunctionLibrary.SpawnSystemAtLocation` "/Game/StudentWork/Particles/NS_FieryExplosion.NS_FieryExplosion" (`self.K2_GetActorLocation`)))

(event `self.ReceiveAnyDamage`
  (params (Damage :type "Float (single-precision)") (DamageType :type "DamageType Object Reference") (InstigatedBy :type "Controller Object Reference") (DamageCauser :type "Actor Object Reference"))
  ;[1 0.05092 0.03103] Minion actions
  ;;[1 1 1] Minion takes damage
  (if (not (`self.bMinionDead`))
    (bind _output_get (set `self.MinionCurrentHealth` (- (`self.MinionCurrentHealth`) Damage)))
    (`KismetSystemLibrary.PrintString` (`KismetStringLibrary.Conv_DoubleToString` _output_get) true true (struct :`R` 1.0 :`G` 0.007351 :`B` 0.473541 :`A` 1.0))
    (`/Engine/EditorBlueprintResources/StandardMacros.IsValid` (`self.MinionHealthBarRef`) ; Checks if ref to EnemyHealthBar widget\nexists yet to avoid runtime error
      (:`Is Valid`
        (set `/Game/StudentWork/UI/WBP_EnemyHealthBar.Health` _output_get (`self.MinionHealthBarRef`)) ; Sets health in enemy's visible\nhealth bar
      )
      (:`Is Not Valid`
        _))
    (`self.ChangeMinionColourToRed`)
    (if (<= (`self.MinionCurrentHealth`) 0.0)
      (`self.MinionDies`)
      (set `self.bEnemyDetected` false))))

(event `AimAtEnemy`
  (bind _turret (`self.Turret`))
  ;[1 0.05092 0.03103] Minion actions
  ;;[1 1 1] Minion aims at enemy
  (bind _target (`self.Target`)
    (:`then`
      (`SceneComponent.K2_SetWorldRotation` _turret (`KismetMathLibrary.FindLookAtRotation` (`SceneComponent.K2_GetComponentLocation` _turret) (`self.K2_GetActorLocation` _target)) false false))
    (:`else`)))

(event `HullToFace`
  (bind _returnvalue (`self.GetVelocity`))
  (bind _tank (`self.Tank`))
  (bind (_returnvalue_roll _returnvalue_pitch _returnvalue_yaw) (`KismetMathLibrary.BreakRotator` (`KismetMathLibrary.MakeRotFromX` _returnvalue)))
  ;[1 0.05092 0.03103] Minion actions
  ;;[1 1 1] Hull to face - makes enemy's body rotate smoothly. Will only rotate if it is moving
  (if (> (`KismetMathLibrary.VSize` _returnvalue) 0.0)
    (`SceneComponent.K2_SetWorldRotation` _tank (`KismetMathLibrary.RInterpTo` (`SceneComponent.K2_GetComponentRotation` _tank) (`KismetMathLibrary.MakeRotator` 0.0 0.0 _returnvalue_yaw) (`GameplayStatics.GetWorldDeltaSeconds`) 2.0) false false)))

(event `self.ReceiveTick`
  (params (DeltaSeconds :type "Float (single-precision)"))
  ;[1 0.05092 0.03103] Minion actions
  ;;[1 1 1] Minion aims at enemy
  (`self.AimAtEnemy`)
  (`self.HullToFace`))

(event `self.ReceiveBeginPlay`
  ;[1 0 0] Event BeginPlay
  (`|ExecutionSequence`
    (:`then_0`
      ;[0 1 0.7967] Widgets
      ;;[1 1 1] Creates reference for minion health bar widget
      (bind _aswbp_enemy_health_bar (cast `/Game/StudentWork/UI/WBP_EnemyHealthBar` (`WidgetComponent.GetUserWidgetObject` (`self.HealthWidget`))))
      (set `self.MinionHealthBarRef` _aswbp_enemy_health_bar))
    (:`then_1`
      ;;[1 1 1] Sets up overlay material and the overlay material's flashing speed
      (`MeshComponent.SetOverlayMaterial` (`self.Tank`) (`self.DamageOverlayMat`))
      (`MeshComponent.SetOverlayMaterial` (`self.Turret`) (`self.DamageOverlayMat`))
      (`TimelineComponent.SetPlayRate` (`self.Flash`) (`self.FlashMultiplier`)))
    (:`then_2`
      (bind _outactors (`GameplayStatics.GetAllActorsOfClassWithTag` "/Script/Engine.Actor" "Enemy"))
      (for _array_element _outactors
        (`KismetArrayLibrary.Array_Add` (`self.EnemyArr`) _array_element)))))

(event `self.MinionHealthBarVisibilitySensor.OnComponentBeginOverlap`
  (params (OverlappedComponent :type "PrimitiveComponent Object Reference") (OtherActor :type "Actor Object Reference") (OtherComp :type "PrimitiveComponent Object Reference") (OtherBodyIndex :type Integer) (bFromSweep :type Boolean) (SweepResult :type "HitResult Structure (by ref)"))
  ;[0 1 0.7967] Widgets
  ;;[1 1 1] Minion health bar appears when player is overlapping with the EnemyHealthBarVisibilitySensor
  (cast `/Game/StudentWork/Blueprints/BP_PlayerCharacter` OtherActor)
  (`SceneComponent.SetVisibility` (`self.HealthWidget`) true false))

(event `self.MinionHealthBarVisibilitySensor.OnComponentEndOverlap`
  (params (OverlappedComponent :type "PrimitiveComponent Object Reference") (OtherActor :type "Actor Object Reference") (OtherComp :type "PrimitiveComponent Object Reference") (OtherBodyIndex :type Integer))
  ;[0 1 0.7967] Widgets
  ;;[1 1 1] Minion health bar appears when player is overlapping with the EnemyHealthBarVisibilitySensor
  (cast `/Game/StudentWork/Blueprints/BP_PlayerCharacter` OtherActor)
  (`SceneComponent.SetVisibility` (`self.HealthWidget`) false false))

(fn `UserConstructionScript`
  (`SceneComponent.K2_SetWorldRotation` (`self.Tank`) (`SceneComponent.K2_GetComponentRotation` (`self.CapsuleComponent`)) false false)
  (bind _returnvalue (`KismetMaterialLibrary.CreateDynamicMaterialInstance` "/Game/StudentWork/Materials/M_DamageOverlay.M_DamageOverlay"))
  (set `self.DamageOverlayMat` _returnvalue))