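; Rotating bridge puzzle actor that swings its pivot's yaw back and forth between -90 and 90 degrees.
; Each MoveBridge event waits briefly, then adds RotationDirection to the yaw, clamped to those limits; the interp settings make this an instant step.
; A limit check then flags the end reached and reverses the direction in 45-degree increments, printing debug strings.
; Nothing in this graph calls MoveBridge.
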(event `MoveBridge`
  (bind _pivotpoint (`self.PivotPoint`))
  (bind _returnvalue (`SceneComponent.K2_GetComponentRotation` _pivotpoint))
  (`KismetSystemLibrary.Delay` 0.25)
  (`SceneComponent.K2_SetWorldRotation` _pivotpoint (`KismetMathLibrary.RInterpTo` _returnvalue (`KismetMathLibrary.MakeRotator` 0.0 0.0 (`KismetMathLibrary.FClamp` (+ (.yaw _returnvalue) (`self.RotationDirection`)) -90.0 90.0)) 1.0 1.0) false false)
  (`self.CheckIfRotationLimitReached`))

(event `CheckIfRotationLimitReached`
  (if (== (.yaw (`SceneComponent.K2_GetComponentRotation` (`self.PivotPoint`))) 90.0)
    (set `self.bLeftMostLimitReached` false)
    (set `self.bRightMostLimitReached` true)
    (`self.SetNewDirection` :!label _label)
    (elif (== (.yaw (`SceneComponent.K2_GetComponentRotation` (`self.PivotPoint`))) -90.0)
      (set `self.bRightMostLimitReached` false)
      (set `self.bLeftMostLimitReached` true)
      (goto _label))))

(event `SetNewDirection`
  (if (`self.bRightMostLimitReached`)
    (`KismetSystemLibrary.PrintString` "right most limit reached")
    (set `self.RotationDirection` -45.0) ; Sets direction to go -45 degrees (so, left)
    (else
      (`KismetSystemLibrary.PrintString` "right most limit NOT reached")
      (if (`self.bLeftMostLimitReached`)
        (`KismetSystemLibrary.PrintString` "left most limit reached")
        (set `self.RotationDirection` 45.0) ; Sets direction to go 45 degrees (so, right)
        (else
          (`KismetSystemLibrary.PrintString` "left most limit NOT reached"))))))

(fn `UserConstructionScript`)