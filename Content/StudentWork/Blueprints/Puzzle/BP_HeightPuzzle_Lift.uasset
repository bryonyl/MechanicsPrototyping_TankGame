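; Lift platform for a height puzzle, driven by an InterpToMovement component, apparently unfinished.
; BeginPlay increments and prints PlatformID.
; Component activation starts a one-second timer with no bound event, then feeds a random height into the first control point's Z via struct and vector setters, printing a random height for debugging.
; The second control point's handling sets no new values and ends in an empty zero-position check.
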(event `self.ReceiveBeginPlay`
  (bind _result (`/Engine/EditorBlueprintResources/StandardMacros.IncrementInt` (`self.PlatformID`))
    (:`  `
      (bind _output_get (set `self.PlatformID` _result)) ; increment platform id by 1
      (`KismetSystemLibrary.PrintString` (`KismetStringLibrary.Conv_IntToString` _output_get)))))

(event `DelayMovement`
  (`KismetSystemLibrary.K2_SetTimerDelegate` :`Time` 1.0))

(event `self.InterpToMovement.OnComponentActivated`
  (params (Component :type "ActorComponent Object Reference") (bReset :type Boolean))
  (bind _returnvalue (`KismetMathLibrary.RandomFloatInRange` 300.0 500.0))
  (`self.DelayMovement`)
  (`|ExecutionSequence`
    (:`then_0`
      (bind _structout (setmembers `InterpControlPoint` :`StructRef` (`|GetArrayItem` (`InterpToMovementComponent.ControlPoints` (`self.InterpToMovement`)))))
      (`KismetMathLibrary.Vector_Set` (`.PositionControlPoint` (break `InterpControlPoint` _structout)) 0.0 0.0 _returnvalue)
      (`KismetSystemLibrary.PrintString` (`KismetStringLibrary.Conv_DoubleToString` _returnvalue)))
    (:`then_1`
      (bind _structout_2 (setmembers `InterpControlPoint` :`StructRef` (`|GetArrayItem` (`InterpToMovementComponent.ControlPoints` (`self.InterpToMovement`)) 1)))
      (bind _positioncontrolpoint (break `InterpControlPoint` _structout_2))
      (`KismetMathLibrary.Vector_Set` _positioncontrolpoint)
      (if (== _positioncontrolpoint (0.0 0.0 0.0))
        _))))

(fn `UserConstructionScript`)