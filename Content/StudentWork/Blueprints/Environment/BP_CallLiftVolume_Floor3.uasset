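; Interactable call volume that summons the Floor 3 lift platform to its own floor.
; On BeginPlay it finds and caches the BP_LiftPlatform_Main_Floor3 actor in the world.
; Interact writes the volume's ThisFloor value into DesiredFloor on that platform's widget, then calls MoveLiftPlatform, so the widget carries the destination.
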(event `self.ReceiveBeginPlay`
  (bind _returnvalue (`GameplayStatics.GetActorOfClass` "/Game/StudentWork/Blueprints/Environment/BP_LiftPlatform_Main_Floor3.BP_LiftPlatform_Main_Floor3_C"))
  (set `self.Level3LiftPlatformRef` _returnvalue))

(event `/Game/StudentWork/BI_Interaction.Interact`
  (bind _level3liftplatformref (`self.Level3LiftPlatformRef`))
  (bind _output_get (set `self.ThisFloor` (`self.ThisFloor`)))
  (set `/Game/StudentWork/UI/Menus/WBP_LiftControls_Level3.DesiredFloor` _output_get (`/Game/StudentWork/Blueprints/Environment/BP_LiftPlatform_Main_Floor3.GetLevel3LiftPlatformWidget` _level3liftplatformref))
  (`/Game/StudentWork/Blueprints/Environment/BP_LiftPlatform_Main.MoveLiftPlatform` _level3liftplatformref))

(fn `UserConstructionScript`
  (`parent.UserConstructionScript`))