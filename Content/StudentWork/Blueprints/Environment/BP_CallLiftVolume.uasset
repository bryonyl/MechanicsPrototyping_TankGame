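; BP_CallLiftVolume is an interactable that calls the main lift platform to the floor set in its ThisFloor variable.
; On BeginPlay it caches the BP_LiftPlatform_Main actor found with GetActorOfClass.
; Interact writes ThisFloor into the lift controls widget's DesiredFloor, then triggers MoveLiftPlatform on the platform.
; PickUpItem is only a stub that returns an empty value.
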(event `self.ReceiveBeginPlay`
  (bind _returnvalue (`GameplayStatics.GetActorOfClass` "/Game/StudentWork/Blueprints/Environment/BP_LiftPlatform_Main.BP_LiftPlatform_Main_C"))
  (set `self.MainLiftPlatformRef` _returnvalue))

(event `/Game/StudentWork/BI_Interaction.Interact`
  (bind _mainliftplatformref (`self.MainLiftPlatformRef`))
  (bind _output_get (set `self.ThisFloor` (`self.ThisFloor`)))
  (set `/Game/StudentWork/UI/Menus/WBP_LiftControls_Main.DesiredFloor` _output_get (`/Game/StudentWork/Blueprints/Environment/BP_LiftPlatform_Main.GetLiftControlsWidget` _mainliftplatformref))
  (`/Game/StudentWork/Blueprints/Environment/BP_LiftPlatform_Main.MoveLiftPlatform` _mainliftplatformref))

(fn `PickUpItem`
  (returns (Item :type String))
  (return ""))

(fn `UserConstructionScript`)