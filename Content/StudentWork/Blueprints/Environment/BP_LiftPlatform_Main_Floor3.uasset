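; Lift platform Blueprint for floor 3 that lets the player choose a floor from an on-screen control widget.
; Overlapping the sensor shows a cursor, opens a cached WBP_LiftControls_Level3 widget and starts a use-allowed timer; leaving removes it and restores game input.
; MoveLiftPlatform matches the widget's DesiredFloor to an index in AllFloors, then a timeline lerps the platform's relative location to that floor.
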(event `self.PlayerCollisionSensor.OnComponentBeginOverlap`
  (params (OverlappedComponent :type "PrimitiveComponent Object Reference") (OtherActor :type "Actor Object Reference") (OtherComp :type "PrimitiveComponent Object Reference") (OtherBodyIndex :type Integer) (bFromSweep :type Boolean) (SweepResult :type "HitResult Structure (by ref)"))
  (bind _returnvalue (`GameplayStatics.GetPlayerController` 0))
  (set `self.OverlappedActor` OtherActor)
  (`WidgetBlueprintLibrary.SetInputMode_GameAndUIEx` _returnvalue null)
  (set `PlayerController.bShowMouseCursor` true _returnvalue)
  (bind _level3liftcontrolswidgetref (`self.Level3LiftControlsWidgetRef`)
    (:`then`
      _)
    (:`else`
      (bind _returnvalue_2 (`|CreateWidget` "/Game/StudentWork/UI/Menus/WBP_LiftControls_Level3.WBP_LiftControls_Level3_C"))
      (set `self.Level3LiftControlsWidgetRef` _returnvalue_2)))
  (`UserWidget.AddToViewport` _level3liftcontrolswidgetref 0)
  (`self.StartLiftUseAllowedTimer`))

(event `self.PlayerCollisionSensor.OnComponentEndOverlap`
  (params (OverlappedComponent :type "PrimitiveComponent Object Reference") (OtherActor :type "Actor Object Reference") (OtherComp :type "PrimitiveComponent Object Reference") (OtherBodyIndex :type Integer))
  (bind _returnvalue (`GameplayStatics.GetPlayerController` 0))
  (`WidgetBlueprintLibrary.SetInputMode_GameOnly` _returnvalue)
  (set `PlayerController.bShowMouseCursor` false _returnvalue)
  (`Widget.RemoveFromParent` (`self.Level3LiftControlsWidgetRef`))
  (set `self.bLiftUseAllowed` false))

(event `self.MoveLiftPlatform`
  (for (_array_element _array_index) (`self.AllFloors`)
    (if (== (`/Game/StudentWork/UI/Menus/WBP_LiftControls_Level3.DesiredFloor` (`self.Level3LiftControlsWidgetRef`)) _array_index)
      (set `self.StartLocation` (`SceneComponent.RelativeLocation` (`self.Platform`)))
      (set `self.TargetLocation` _array_element)))
  (bind (_direction _newtrack_0) (`Timeline|Timeline_0` :!via `PlayFromStart`)
    (:`Update`
      (`SceneComponent.K2_SetRelativeLocation` (`self.Platform`) (`KismetMathLibrary.VLerp` (`self.StartLocation`) (`self.TargetLocation`) _newtrack_0) false false))))

(fn `GetLevel3LiftPlatformWidget`
  (returns (Level3LiftControlsWidgetRef :type "/Game/StudentWork/UI/Menus/WBP_LiftControls_Level3 Object Reference"))
  (return (`self.Level3LiftControlsWidgetRef`)))

(fn `UserConstructionScript`
  (`parent.UserConstructionScript`))