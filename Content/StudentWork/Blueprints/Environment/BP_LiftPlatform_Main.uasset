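; Lift platform that moves between preset floor locations chosen through a WBP_LiftControls_Main widget.
; Overlapping the sensor shows the widget and mouse cursor and starts a looping timer that allows use for the player or minion; leaving reverses this, though the timer keeps running.
; MoveLiftPlatform lerps the platform to the desired floor with a Timeline.
; A separate event teleports the unlocked minion to the player; passenger snap/unsnap events are empty, their logic disconnected.
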(event `self.ReceiveBeginPlay`
  (bind _returnvalue (`GameplayStatics.GetActorOfClass` "/Game/StudentWork/Blueprints/Minions/BP_Minion_Parent.BP_Minion_Parent_C"))
  (set `self.MinionRef` _returnvalue)
  (bind _returnvalue_2 (`|CreateWidget` "/Game/StudentWork/UI/Menus/WBP_LiftControls_Main.WBP_LiftControls_Main_C"))
  (set `self.LiftControlsWidgetRef` _returnvalue_2))

(event `UnsnapPassengersFromLift`)

(event `SnapPassengersToLift`)

(event `StartLiftUseAllowedTimer`
  (`KismetSystemLibrary.K2_SetTimerDelegate` (delegate `CheckIfLiftUseAllowed`) (`self.LiftUseAllowedTimer`) true))

(event `CheckIfLiftUseAllowed`
  (bind _overlappedactor (`self.OverlappedActor`))
  (if (== _overlappedactor (`GameplayStatics.GetPlayerCharacter` 0))
    (set `self.bLiftUseAllowed` true :!label _label)
    (elif (== _overlappedactor (`self.MinionRef`))
      (goto _label))))

(event `self.PlayerCollisionSensor.OnComponentBeginOverlap`
  (params (OverlappedComponent :type "PrimitiveComponent Object Reference") (OtherActor :type "Actor Object Reference") (OtherComp :type "PrimitiveComponent Object Reference") (OtherBodyIndex :type Integer) (bFromSweep :type Boolean) (SweepResult :type "HitResult Structure (by ref)"))
  (bind _returnvalue (`GameplayStatics.GetPlayerController` 0))
  (set `self.OverlappedActor` OtherActor)
  (`WidgetBlueprintLibrary.SetInputMode_GameAndUIEx` _returnvalue null)
  (set `PlayerController.bShowMouseCursor` true _returnvalue)
  (bind _liftcontrolswidgetref (`self.LiftControlsWidgetRef`)
    (:`then`
      _)
    (:`else`
      (bind _returnvalue_2 (`|CreateWidget` "/Game/StudentWork/UI/Menus/WBP_LiftControls_Main.WBP_LiftControls_Main_C"))
      (set `self.LiftControlsWidgetRef` _returnvalue_2)))
  (`UserWidget.AddToViewport` _liftcontrolswidgetref 0)
  (`self.StartLiftUseAllowedTimer`))

(event `self.PlayerCollisionSensor.OnComponentEndOverlap`
  (params (OverlappedComponent :type "PrimitiveComponent Object Reference") (OtherActor :type "Actor Object Reference") (OtherComp :type "PrimitiveComponent Object Reference") (OtherBodyIndex :type Integer))
  (bind _returnvalue (`GameplayStatics.GetPlayerController` 0))
  (`WidgetBlueprintLibrary.SetInputMode_GameOnly` _returnvalue)
  (set `PlayerController.bShowMouseCursor` false _returnvalue)
  (`Widget.RemoveFromParent` (`self.LiftControlsWidgetRef`))
  (set `self.bLiftUseAllowed` false))

(event `MoveLiftPlatform`
  (for (_array_element _array_index) (`self.AllFloors`)
    (if (== (`/Game/StudentWork/UI/Menus/WBP_LiftControls_Main.DesiredFloor` (`self.LiftControlsWidgetRef`)) _array_index)
      (set `self.StartLocation` (`SceneComponent.RelativeLocation` (`self.Platform`)))
      (set `self.TargetLocation` _array_element)))
  (bind (_direction _newtrack_0) (`Timeline|Timeline` :!via `PlayFromStart`)
    (:`Update`
      (`SceneComponent.K2_SetRelativeLocation` (`self.Platform`) (`KismetMathLibrary.VLerp` (`self.StartLocation`) (`self.TargetLocation`) _newtrack_0) false false))))

(event `TeleportMinionToPlayer`
  (bind _minionref (`self.MinionRef`))
  (if (`/Game/StudentWork/Blueprints/Minions/BP_Minion_Parent.bMinionUnlocked` _minionref)
    (`self.K2_TeleportTo` :`self` _minionref :`DestLocation` (`self.K2_GetActorLocation` (`GameplayStatics.GetPlayerCharacter` 0)))))

(fn `GetLiftControlsWidget`
  (returns (LiftControlsWidgetRef :type "/Game/StudentWork/UI/Menus/WBP_LiftControls_Main Object Reference"))
  (return (`self.LiftControlsWidgetRef`)))

(fn `UserConstructionScript`)