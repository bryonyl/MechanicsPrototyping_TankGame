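; Interactable sliding double door that can be locked and optionally gated by a keycard.
; BeginPlay sets the lock state, shown by red or green indicator materials and point lights.
; Interact briefly shows a locked prompt if the required keycard is missing; otherwise, unless moving, it turns the lights green and toggles the door.
; A FlipFlop plays or reverses a Timeline that slides both panels and swaps the open/close prompt text.
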(event `self.ReceiveBeginPlay`
  ;[1 1 1] Creating a reference to player controller for later use
  (bind _asbp_mech_player_controller (cast `/Game/StudentWork/Blueprints/BP_MechPlayerController` (`GameplayStatics.GetPlayerController` 0)))
  (set `self.PlayerControllerRef` _asbp_mech_player_controller)
  ;[1 1 1] Doors are set up when the game starts
  (if (`self.bDoorLocked`)
    (`self.SetDoorLocked`)
    (else
      (`self.SetDoorUnlocked`))))

(event `AllowOpenAndCloseDoor`
  (bind _ac_interactable (`self.AC_Interactable`))
  ;[1 1 1] Opening and closing of the door
  (`/Engine/EditorBlueprintResources/StandardMacros.FlipFlop`
    (:`A`
      (set `/Game/StudentWork/Blueprints/AC_Interactable.CustomInteractPromptText` "[E] Close Door" _ac_interactable)
      (set `self.bDoorMoving` true)
      (bind (_direction _rightdoormovementtrack _leftdoormovementtrack) (`Timeline|Timeline` :!label _label)
        (:`Update`
          (`SceneComponent.K2_SetRelativeLocation` (`self.RightDoor`) _rightdoormovementtrack false false)
          (`SceneComponent.K2_SetRelativeLocation` (`self.LeftDoor`) _leftdoormovementtrack false false))
        (:`Finished`
          (set `self.bDoorMoving` false))))
    (:`B`
      (set `/Game/StudentWork/Blueprints/AC_Interactable.CustomInteractPromptText` "[E] Open Door" _ac_interactable)
      (set `self.bDoorMoving` true)
      (goto _label :!via `Reverse`))))

(event `/Game/StudentWork/BI_Interaction.Interact`
  ;[1 1 1] Player interaction with door
  (if (`self.bDoorLocked`)
    (if (`self.bDoorUsesKeycardForUnlock`)
      (if (`self.bPlayerHasKeycardRequired`)
        (if (not (`self.bDoorMoving`)) :!label _label_2
          (`self.SetDoorLightIndicatorsUnlocked`)
          (`self.AllowOpenAndCloseDoor`))
        (else
          (bind _playercharacterref (`self.PlayerCharacterRef`)
            (:`then`
              _)
            (:`else`
              (bind _asbp_player_character (cast `/Game/StudentWork/Blueprints/BP_PlayerCharacter` (`GameplayStatics.GetPlayerCharacter` 0)))
              (bind _output_get (set `self.PlayerCharacterRef` _asbp_player_character))))
          (`/Game/StudentWork/UI/WBP_InteractPrompt.UpdateInteractPromptText` (`/Game/StudentWork/Blueprints/BP_PlayerCharacter.InteractPromptRef` _output_get) "Door is Locked!")
          (`/Game/StudentWork/UI/WBP_InteractPrompt.UpdateInteractPromptText` (`/Game/StudentWork/Blueprints/BP_PlayerCharacter.InteractPromptRef` _playercharacterref) "Door is Locked!")
          (`KismetSystemLibrary.Delay` 1.0)
          (`/Game/StudentWork/UI/WBP_InteractPrompt.UpdateInteractPromptText` (`/Game/StudentWork/Blueprints/BP_PlayerCharacter.InteractPromptRef` _playercharacterref) "[E] Open Door")))
      (else
        (goto _label_2)))
    (else
      (goto _label_2))))

(event `SetDoorLocked`
  ;[1 1 1] Lock Door
  (set `self.bDoorLocked` true)
  (set `/Game/StudentWork/Blueprints/AC_Interactable.CustomInteractPromptText` "[E] Open Door" (`self.AC_Interactable`))
  (`self.SetDoorLightIndicatorsLocked`))

(event `SetDoorLightIndicatorsLocked`
  ;[1 1 1] Door light indicators are set to locked with a red light
  (`PrimitiveComponent.SetMaterial` (`self.LightIndicatorExterior`) 1 "/Game/Materials/MI_EmissiveRed.MI_EmissiveRed")
  (`PrimitiveComponent.SetMaterial` (`self.LightIndicatorInterior`) 1 "/Game/Materials/MI_EmissiveRed.MI_EmissiveRed")
  (`LightComponent.SetLightColor` (`self.LightIndicatorExteriorPointLight`) (struct :`R` 0.693 :`G` 0.016221 :`A` 1.0) true)
  (`LightComponent.SetLightColor` (`self.LightIndicatorInteriorPointLight`) (struct :`R` 0.693 :`G` 0.016221 :`A` 1.0) true))

(event `SetDoorUnlocked`
  ;[1 1 1] Unlock Door
  (set `self.bDoorLocked` false)
  (set `/Game/StudentWork/Blueprints/AC_Interactable.CustomInteractPromptText` "[E] Open Door" (`self.AC_Interactable`))
  (`self.SetDoorLightIndicatorsUnlocked`))

(event `SetDoorLightIndicatorsUnlocked`
  ;[1 1 1] Door light indicators are set to unlocked with a green light
  (`PrimitiveComponent.SetMaterial` (`self.LightIndicatorExterior`) 1 "/Game/Materials/MI_Green_Emissive.MI_Green_Emissive")
  (`PrimitiveComponent.SetMaterial` (`self.LightIndicatorInterior`) 1 "/Game/Materials/MI_Green_Emissive.MI_Green_Emissive")
  (`LightComponent.SetLightColor` (`self.LightIndicatorExteriorPointLight`) (struct :`R` 0.137255 :`G` 1.0 :`B` 0.035294 :`A` 1.0) true)
  (`LightComponent.SetLightColor` (`self.LightIndicatorInteriorPointLight`) (struct :`R` 0.137255 :`G` 1.0 :`B` 0.035294 :`A` 1.0) true))

(fn `PickUpItem`
  (returns (Item :type String))
  (return ""))

(fn `UserConstructionScript`)