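; Explosive projectile that detonates after a flashing warning, triggered by a hit on its sphere mesh or a timer started at BeginPlay.
; A timeline drives the flash level on a dynamic material created in the construction script.
; When it finishes, a sphere trace damages nearby actors, destroys those tagged Explodable, then replaces the projectile with a fiery Niagara explosion.
; The trace leaves persistent debug drawing.
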(event `self.ReceiveBeginPlay`
  ;[1 1 1] Timer before Explode event starts
  (`KismetSystemLibrary.K2_SetTimerDelegate` (delegate `Explode`) 3.0))

(event `self.SM_Sphere.OnComponentHit`
  (params (HitComponent :type "PrimitiveComponent Object Reference") (OtherActor :type "Actor Object Reference") (OtherComp :type "PrimitiveComponent Object Reference") (NormalImpulse :type "Vector Structure") (Hit :type "HitResult Structure (by ref)"))
  ;[1 1 1] When the projectile collides with something, set off the Explode effect
  (`self.Explode`))

(event `Explode`
  (bind _returnvalue (`self.K2_GetActorLocation`))
  ;[1 1 1] Flashing material
  (bind (_direction _flash) (`Timeline|Timeline`)
    (:`Update`
      (`MaterialInstanceDynamic.SetScalarParameterValue` (`self.FlashMaterial`) "FlashLevel" _flash))
    (:`Finished`
      ;[1 1 1] Multiple explosions possible via Multi Sphere Trace By Channel (for example, if multiple explodable objects are in proximity of each other). Particle systems spawned after the projectile is destroyed
      (bind _outhits (`KismetSystemLibrary.SphereTraceMulti` :`Start` _returnvalue :`End` _returnvalue :`Radius` 100.0 :`TraceChannel` "TraceTypeQuery1" :`DrawDebugType` "Persistent"))
      (for _array_element _outhits
        (bind (_bblockinghit _binitialoverlap _time _distance _location _impactpoint _normal _impactnormal _physmat _hitactor) (`GameplayStatics.BreakHitResult` _array_element))
        ;[1 1 1] If the hit actor has the tag "Explodable", then it will be destroyed. If not, then it will just have damage applied to it
        (if (`self.ActorHasTag` _hitactor "Explodable")
          (`GameplayStatics.ApplyDamage` _hitactor 25.0)
          (`self.K2_DestroyActor` _hitactor)
          (else
            (`GameplayStatics.ApplyDamage` _hitactor 25.0))))
      (`self.K2_DestroyActor`)
      (`NiagaraFunctionLibrary.SpawnSystemAtLocation` "/Game/StudentWork/Particles/NS_FieryExplosion.NS_FieryExplosion" (`self.K2_GetActorLocation`)))))

(fn `UserConstructionScript`
  (bind _returnvalue (`PrimitiveComponent.CreateDynamicMaterialInstance` (`self.SM_Sphere`) 0 "/Game/StudentWork/Materials/M_ControlledFlash_Red.M_ControlledFlash_Red" "None")) ; Replaces Element 0 Material, which is the main material
  (set `self.FlashMaterial` _returnvalue))