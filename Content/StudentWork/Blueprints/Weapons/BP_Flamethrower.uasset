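; Flamethrower weapon for a tank that deals repeated small damage along a short line in front of it while fire is held.
; Pressing fire spawns an attached Niagara flame on the tank's DirectionArrow, and releasing deactivates it.
; While triggered, a multi-sphere object trace runs forward from that arrow and damages every hit actor, rate-limited by a brief timer-reset cooldown.
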(event `self.Triggered`
  (bind _directionarrow (`/Game/StudentWork/Blueprints/BP_PlayerCharacter.DirectionArrow` (`self.MyTank`)))
  (bind _returnvalue_location (`KismetMathLibrary.BreakTransform` (`SceneComponent.K2_GetComponentToWorld` _directionarrow)))
  (if (not (`self.bCooldown`))
    (bind _outhits (`KismetSystemLibrary.SphereTraceMultiForObjects` (0.0 0.0 0.0) (+ _returnvalue_location (* (`SceneComponent.GetForwardVector` _directionarrow) 200.0)) 0.0 (`self.Object Types`)))
    (for _array_element _outhits
      (`GameplayStatics.ApplyDamage` (`.HitActor` (`GameplayStatics.BreakHitResult` _array_element)) 2.0))
    (set `self.bCooldown` true)
    (`KismetSystemLibrary.K2_SetTimerDelegate` (delegate `ResetCooldown`) 0.2)))

(event `ResetCooldown`
  (set `self.bCooldown` false))

(event `self.Started`
  (bind _returnvalue (`NiagaraFunctionLibrary.SpawnSystemAttached` "/Game/StudentWork/Particles/NS_FlameSpurt.NS_FlameSpurt" (`/Game/StudentWork/Blueprints/BP_PlayerCharacter.DirectionArrow` (`self.MyTank`)) "None" (0.0 0.0 0.0) (struct) "KeepRelativeOffset"))
  (set `self.FlameSystem` _returnvalue))

(event `self.Completed`
  (`ActorComponent.Deactivate` (`self.FlameSystem`)))

(fn `UserConstructionScript`
  (`parent.UserConstructionScript`))