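; BP_LaserSMG is a rapid-fire tank weapon that shoots small, fast projectiles.
; When triggered off cooldown, it spawns a BP_SmallFastProjectile at the location and rotation of the owning tank's DirectionArrow.
; A boolean cooldown, cleared by a short timer event, caps the fire rate.
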(event `self.Triggered`
  (bind _directionarrow (`/Game/StudentWork/Blueprints/BP_PlayerCharacter.DirectionArrow` (`self.MyTank`)))
  (if (not (`self.bCooldown`))
    (`|SpawnActorFromClass` "/Game/StudentWork/Blueprints/Weapons/BP_SmallFastProjectile.BP_SmallFastProjectile_C" (`KismetMathLibrary.MakeTransform` (`SceneComponent.K2_GetComponentLocation` _directionarrow) (`SceneComponent.K2_GetComponentRotation` _directionarrow)) "Undefined" "MultiplyWithRoot" null null) ; Collision Handling Override = what should happen if I try to spawn this actor but something else is in the way
    (set `self.bCooldown` true)
    (`KismetSystemLibrary.K2_SetTimerDelegate` (delegate `EndCooldown`) 0.1)))

(event `EndCooldown`
  (set `self.bCooldown` false))

(fn `UserConstructionScript`
  (`parent.UserConstructionScript`))