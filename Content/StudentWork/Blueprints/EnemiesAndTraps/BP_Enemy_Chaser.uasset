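; BP_Enemy_Chaser is an enemy that pursues the player and fires projectiles.
; Its Move event uses AIMoveTo to approach the player character reference, when valid, with an acceptance radius that keeps it at some distance.
; Its Attack event spawns a BP_EnemyProjectile at the FirePoint component's world location and rotation.
; The construction script only calls the parent's, and nothing in this file triggers Move or Attack.
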(event `self.Move`
  (`/Engine/EditorBlueprintResources/StandardMacros.IsValid` (`self.PlayerCharacterRef`)
    (:`Is Valid`
      (`|AIMoveTo` self (0.0 0.0 0.0) (`self.PlayerCharacterRef`) 350.0))))

(event `self.Attack`
  (bind _firepoint (`self.FirePoint`))
  (`|SpawnActorFromClass` "/Game/StudentWork/Blueprints/EnemiesAndTraps/BP_EnemyProjectile.BP_EnemyProjectile_C" (`KismetMathLibrary.MakeTransform` (`SceneComponent.K2_GetComponentLocation` _firepoint) (`SceneComponent.K2_GetComponentRotation` _firepoint)) "Undefined" "MultiplyWithRoot" null null))

(fn `UserConstructionScript`
  (`parent.UserConstructionScript`))