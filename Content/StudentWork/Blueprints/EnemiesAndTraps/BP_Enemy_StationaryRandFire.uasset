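; Stationary-enemy variant, going by its name, that fires projectiles in random directions from three fire points.
; Its Attack event spawns one actor at each point with its own random yaw, using BP_EnemyProjectile_FastWeak for the second and third; the first spawn shows no class.
; BeginPlay calls the parent and stores the points in FirePointArr, which Attack bypasses by referencing each point directly.
; Nothing in this graph triggers Attack, and Tick is empty.
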(event `self.ReceiveTick`
  (params (DeltaSeconds :type "Float (single-precision)")))

(event `self.ReceiveBeginPlay`
  (`parent.ReceiveBeginPlay`)
  (set `self.FirePointArr` (`|MakeArray` (`self.FirePoint`) (`self.FirePoint1`) (`self.FirePoint2`))))

(event `self.Attack`
  (bind (_returnvalue_roll _returnvalue_pitch _returnvalue_yaw) (`KismetMathLibrary.BreakRotator` (`KismetMathLibrary.RandomRotator` false)))
  (bind (_returnvalue_roll_2 _returnvalue_pitch_2 _returnvalue_yaw_2) (`KismetMathLibrary.BreakRotator` (`KismetMathLibrary.RandomRotator` false)))
  (bind (_returnvalue_roll_3 _returnvalue_pitch_3 _returnvalue_yaw_3) (`KismetMathLibrary.BreakRotator` (`KismetMathLibrary.RandomRotator` false)))
  (`|SpawnActorFromClass` "/Game/StudentWork/Blueprints/EnemiesAndTraps/BP_EnemyProjectile_FastWeak.BP_EnemyProjectile_FastWeak_C" (`KismetMathLibrary.MakeTransform` (`SceneComponent.K2_GetComponentLocation` (`self.FirePoint`)) (`KismetMathLibrary.MakeRotator` 0.0 0.0 _returnvalue_yaw_3)) "Undefined" "MultiplyWithRoot" null null)
  (`|SpawnActorFromClass` "/Game/StudentWork/Blueprints/EnemiesAndTraps/BP_EnemyProjectile_FastWeak.BP_EnemyProjectile_FastWeak_C" (`KismetMathLibrary.MakeTransform` (`SceneComponent.K2_GetComponentLocation` (`self.FirePoint1`)) (`KismetMathLibrary.MakeRotator` 0.0 0.0 _returnvalue_yaw)) "Undefined" "MultiplyWithRoot" null null)
  (`|SpawnActorFromClass` "/Game/StudentWork/Blueprints/EnemiesAndTraps/BP_EnemyProjectile_FastWeak.BP_EnemyProjectile_FastWeak_C" (`KismetMathLibrary.MakeTransform` (`SceneComponent.K2_GetComponentLocation` (`self.FirePoint2`)) (`KismetMathLibrary.MakeRotator` 0.0 0.0 _returnvalue_yaw_2)) "Undefined" "MultiplyWithRoot" null null))

(fn `UserConstructionScript`
  (`parent.UserConstructionScript`))