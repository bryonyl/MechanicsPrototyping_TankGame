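; Patrolling enemy Blueprint that moves between two waypoints and fires a slow, powerful projectile when it attacks.
; BeginPlay gathers every BP_EnemyWaypoint in the world and starts a movement timer.
; Move uses AIMoveTo behind an IsMoving guard, flipping the target index between 0 and 1 on each successful arrival.
; Attack spawns BP_EnemyProjectile_SlowPowerful at the FirePoint's location and rotation.
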(event `self.ReceiveBeginPlay`
  (`parent.ReceiveBeginPlay`)
  (bind _outactors (`GameplayStatics.GetAllActorsOfClass` "/Game/StudentWork/Blueprints/EnemiesAndTraps/BP_EnemyWaypoint.BP_EnemyWaypoint_C"))
  (bind _output_get (set `self.WaypointsInWorld` _outactors))
  (set `self.TargetWaypoint` (`|GetArrayItem` _output_get (`self.WaypointIndex`)))
  (`self.StartMovementTimer`))

(event `self.Move`
  (if (not (`self.bIsMoving`))
    (set `self.bIsMoving` true)
    (set `self.TargetWaypoint` (`|GetArrayItem` (`self.WaypointsInWorld`) (`self.WaypointIndex`)))
    (`|AIMoveTo` self (0.0 0.0 0.0) (`self.TargetWaypoint`) 350.0
      (:`OnSuccess`
        (set `self.bIsMoving` false)
        (if (== (`self.WaypointIndex`) 1)
          (set `self.WaypointIndex` (- (`self.WaypointIndex`) 1))
          (else
            (set `self.WaypointIndex` (+ (`self.WaypointIndex`) 1))))))))

(event `self.Attack`
  (bind _firepoint (`self.FirePoint`))
  (`|SpawnActorFromClass` "/Game/StudentWork/Blueprints/EnemiesAndTraps/BP_EnemyProjectile_SlowPowerful.BP_EnemyProjectile_SlowPowerful_C" (`KismetMathLibrary.MakeTransform` (`SceneComponent.K2_GetComponentLocation` _firepoint) (`SceneComponent.K2_GetComponentRotation` _firepoint)) "Undefined" "MultiplyWithRoot" null null))

(fn `UserConstructionScript`
  (`parent.UserConstructionScript`))