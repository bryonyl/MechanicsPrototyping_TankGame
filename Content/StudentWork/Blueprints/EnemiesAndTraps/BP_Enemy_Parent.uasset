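; Base enemy tank that detects the player or minions, aims at them and dies in an explosion.
; Sphere overlap flashes a notification and starts looping timers on empty Move and Attack events, left for children.
; Tick turns the turret to stored targets, minion overriding player, and eases the hull toward velocity.
; Damage updates a health bar, shown near the player, and flashes a dynamic overlay material through a timeline.
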(event `self.SphereSensor.OnComponentBeginOverlap`
  (params (OverlappedComponent :type "PrimitiveComponent Object Reference") (OtherActor :type "Actor Object Reference") (OtherComp :type "PrimitiveComponent Object Reference") (OtherBodyIndex :type Integer) (bFromSweep :type Boolean) (SweepResult :type "HitResult Structure (by ref)"))
  ;[0.1063 0.2664 1] Player detection
  ;;[1 1 1] Player character reference is created. Player is detected, movement and attack timers start
  (bind _asbp_player_character (cast `/Game/StudentWork/Blueprints/BP_PlayerCharacter` OtherActor)
    (:`then`
      (set `self.PlayerCharacterRef` _asbp_player_character)
      (set `self.bPlayerDetected` true))
    (:`CastFailed`
      (bind _asbp_minion_parent (cast `/Game/StudentWork/Blueprints/Minions/BP_Minion_Parent` OtherActor))
      (set `self.MinionParentRef` _asbp_minion_parent)
      (set `self.bMinionDetected` true)))
  (`self.ShowPlayerDetectionNotificationWidget`)
  (`self.StartMovementTimer`)
  (`self.StartAttackTimer`))

(event `self.SphereSensor.OnComponentEndOverlap`
  (params (OverlappedComponent :type "PrimitiveComponent Object Reference") (OtherActor :type "Actor Object Reference") (OtherComp :type "PrimitiveComponent Object Reference") (OtherBodyIndex :type Integer))
  ;[0.1063 0.2664 1] Player detection
  ;;[1 1 1] Player is no longer detected
  (bind _asbp_player_character (cast `/Game/StudentWork/Blueprints/BP_PlayerCharacter` OtherActor)
    (:`then`
      (set `self.PlayerCharacterRef` _asbp_player_character)
      (set `self.bPlayerDetected` false))
    (:`CastFailed`
      (bind _asbp_minion_parent (cast `/Game/StudentWork/Blueprints/Minions/BP_Minion_Parent` OtherActor))
      (set `self.MinionParentRef` _asbp_minion_parent)
      (set `self.bMinionDetected` false))))

(event `EnemyDies`
  ;[1 0.05092 0.03103] Enemy actions
  ;;[1 1 1] Enemy dies
  (set `self.bEnemyDead` true)
  (`self.K2_DestroyActor`)
  (`NiagaraFunctionLibrary.SpawnSystemAtLocation` "/Game/StudentWork/Particles/NS_FieryExplosion.NS_FieryExplosion" (`self.K2_GetActorLocation`)))

(event `StartMovementTimer`
  ;[1 0.05092 0.03103] Enemy actions
  ;;[1 1 1] Enemy moves
  (bind _returnvalue (`KismetSystemLibrary.K2_SetTimerDelegate` (delegate `Move`) (`self.MovementUpdateTime`) true))
  (set `self.MovementTimer` _returnvalue))

(event `StartAttackTimer`
  ;[1 0.05092 0.03103] Enemy actions
  ;;[1 1 1] Enemy attacks
  (bind _returnvalue (`KismetSystemLibrary.K2_SetTimerDelegate` (delegate `Attack`) (`self.AttackSpeed`) true))
  (set `self.AttackTimer` _returnvalue))

(event `EnemyDamageFlash`
  ;[1 0.05092 0.03103] Enemy actions
  ;;[1 1 1] Enemy flashes red when damaged
  (`/Engine/EditorBlueprintResources/StandardMacros.DoOnce` false :!label _label
    (:`Completed`
      (bind (_direction _flash) (`Timeline|Flash` :!via `PlayFromStart`)
        (:`Update`
          (`MaterialInstanceDynamic.SetScalarParameterValue` (`self.DamageOverlayMat`) "FlashLevel" _flash))
        (:`Finished`
          (goto _label :!via `Reset`))))))

(event `Move`
  ;[1 0.05092 0.03103] Enemy actions
  ;;[1 1 1] Enemy moves
)

(event `Attack`
  ;[1 0.05092 0.03103] Enemy actions
  ;;[1 1 1] Enemy attacks
)

(event `self.ReceiveAnyDamage`
  (params (Damage :type "Float (single-precision)") (DamageType :type "DamageType Object Reference") (InstigatedBy :type "Controller Object Reference") (DamageCauser :type "Actor Object Reference"))
  ;[1 0.05092 0.03103] Enemy actions
  ;;[1 1 1] Enemy takes damage
  (if (not (`self.bEnemyDead`))
    (bind _output_get (set `self.EnemyCurrentHealth` (- (`self.EnemyCurrentHealth`) Damage)))
    (`KismetSystemLibrary.PrintString` (`KismetStringLibrary.Conv_DoubleToString` _output_get) true true (struct :`R` 0.19867 :`G` 1.0 :`A` 1.0))
    (bind _enemyhealthbarref (`self.EnemyHealthBarRef`)
      (:`then`
        _)
      (:`else`
        (bind _returnvalue (`|CreateWidget` "/Game/StudentWork/UI/WBP_EnemyHealthBar.WBP_EnemyHealthBar_C"))
        (set `self.EnemyHealthBarRef` _returnvalue)))
    (set `/Game/StudentWork/UI/WBP_EnemyHealthBar.Health` _output_get _enemyhealthbarref) ; Sets health in enemy's visible\nhealth bar
    (`self.EnemyDamageFlash`)
    (if (<= (`self.EnemyCurrentHealth`) 0.0)
      (`self.EnemyDies`)
      (set `self.bPlayerDetected` false)
      (set `self.bMinionDetected` false))))

(event `HullToFace`
  (bind _returnvalue (`self.GetVelocity`))
  (bind _tank (`self.Tank`))
  (bind (_returnvalue_roll _returnvalue_pitch _returnvalue_yaw) (`KismetMathLibrary.BreakRotator` (`KismetMathLibrary.MakeRotFromX` _returnvalue)))
  ;[1 0.05092 0.03103] Enemy actions
  ;;[1 1 1] Hull to face - makes enemy's body rotate smoothly. Will only rotate if it is moving
  (if (> (`KismetMathLibrary.VSize` _returnvalue) 0.0)
    (`SceneComponent.K2_SetWorldRotation` _tank (`KismetMathLibrary.RInterpTo` (`SceneComponent.K2_GetComponentRotation` _tank) (`KismetMathLibrary.MakeRotator` 0.0 0.0 _returnvalue_yaw) (`GameplayStatics.GetWorldDeltaSeconds`) 2.0) false false)))

(event `AimAtPlayer`
  (bind _turret (`self.Turret`))
  (bind _playercharacterref (`self.PlayerCharacterRef`))
  ;[1 0.05092 0.03103] Enemy actions
  ;;[1 1 1] Enemy aims at player
  (`/Engine/EditorBlueprintResources/StandardMacros.IsValid` _playercharacterref
    (:`Is Valid`
      (`SceneComponent.K2_SetWorldRotation` _turret (`KismetMathLibrary.FindLookAtRotation` (`SceneComponent.K2_GetComponentLocation` _turret) (`self.K2_GetActorLocation` _playercharacterref)) false false))))

(event `AimAtMinion`
  (bind _turret (`self.Turret`))
  (bind _minionparentref (`self.MinionParentRef`))
  ;[1 0.05092 0.03103] Enemy actions
  ;;[1 1 1] Aim at minion
  (`/Engine/EditorBlueprintResources/StandardMacros.IsValid` _minionparentref
    (:`Is Valid`
      (`SceneComponent.K2_SetWorldRotation` _turret (`KismetMathLibrary.FindLookAtRotation` (`SceneComponent.K2_GetComponentLocation` _turret) (`self.K2_GetActorLocation` _minionparentref)) false false))))

(event `self.ReceiveTick`
  (params (DeltaSeconds :type "Float (single-precision)"))
  ;[1 0.05092 0.03103] Enemy actions
  ;;[1 1 1] Enemy aims at both player and minion on tick
  (`self.AimAtPlayer`)
  (`self.AimAtMinion`)
  (`self.HullToFace`))

(event `self.ReceiveBeginPlay`
  ;[1 0 0] Event BeginPlay
  (`|ExecutionSequence`
    (:`then_0`
      ;[0 1 0.7967] Widgets
      ;;[1 1 1] Creates reference for enemy health bar widget and player detection widget
      (bind _aswbp_enemy_health_bar (cast `/Game/StudentWork/UI/WBP_EnemyHealthBar` (`WidgetComponent.GetUserWidgetObject` (`self.HealthWidget`))))
      (set `self.EnemyHealthBarRef` _aswbp_enemy_health_bar)
      (bind _aswbp_player_detection_notification (cast `/Game/StudentWork/UI/WBP_PlayerDetectionNotification` (`WidgetComponent.GetUserWidgetObject` (`self.PlayerDetectionNotificationWidget`))))
      (set `self.PlayerNotificationDetectionRef` _aswbp_player_detection_notification))
    (:`then_1`
      ;;[1 1 1] Sets up overlay material and the overlay material's flashing speed
      (`MeshComponent.SetOverlayMaterial` (`self.Tank`) (`self.DamageOverlayMat`))
      (`MeshComponent.SetOverlayMaterial` (`self.Turret`) (`self.DamageOverlayMat`))
      (`TimelineComponent.SetPlayRate` (`self.Flash`) (`self.FlashMultiplier`)))))

(event `self.EnemyHealthBarVisibilitySensor.OnComponentBeginOverlap`
  (params (OverlappedComponent :type "PrimitiveComponent Object Reference") (OtherActor :type "Actor Object Reference") (OtherComp :type "PrimitiveComponent Object Reference") (OtherBodyIndex :type Integer) (bFromSweep :type Boolean) (SweepResult :type "HitResult Structure (by ref)"))
  ;[0 1 0.7967] Widgets
  ;;[1 1 1] Enemy bar appears when player is overlapping with the EnemyHealthBarVisibilitySensor
  (cast `/Game/StudentWork/Blueprints/BP_PlayerCharacter` OtherActor)
  (`SceneComponent.SetVisibility` (`self.HealthWidget`) true false))

(event `self.EnemyHealthBarVisibilitySensor.OnComponentEndOverlap`
  (params (OverlappedComponent :type "PrimitiveComponent Object Reference") (OtherActor :type "Actor Object Reference") (OtherComp :type "PrimitiveComponent Object Reference") (OtherBodyIndex :type Integer))
  ;[0 1 0.7967] Widgets
  ;;[1 1 1] Enemy bar appears when player is overlapping with the EnemyHealthBarVisibilitySensor
  (cast `/Game/StudentWork/Blueprints/BP_PlayerCharacter` OtherActor)
  (`SceneComponent.SetVisibility` (`self.HealthWidget`) false false))

(event `ShowPlayerDetectionNotificationWidget`
  (bind _playerdetectionnotificationwidget (`self.PlayerDetectionNotificationWidget`))
  ;[0 1 0.7967] Widgets
  ;;[1 1 1] Shows the player detection notification widget for a short amount of time before hiding it again
  (`SceneComponent.SetVisibility` _playerdetectionnotificationwidget true false)
  (`KismetSystemLibrary.Delay` 0.5)
  (`SceneComponent.SetVisibility` _playerdetectionnotificationwidget false false))

(fn `UserConstructionScript`
  (`SceneComponent.K2_SetWorldRotation` (`self.Tank`) (`SceneComponent.K2_GetComponentRotation` (`self.CapsuleComponent`)) false false)
  (bind _returnvalue (`KismetMaterialLibrary.CreateDynamicMaterialInstance` "/Game/StudentWork/Materials/M_DamageOverlay.M_DamageOverlay"))
  (set `self.DamageOverlayMat` _returnvalue))