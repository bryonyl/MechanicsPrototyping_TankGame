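; BP_Enemy_MoveRandom is an enemy Blueprint that wanders randomly and fires projectiles.
; It overrides the parent's Move event to send an AI move to a random reachable point within a radius around its current location.
; Its Attack override spawns a BP_EnemyProjectile_FastWeak at the FirePoint component's position and rotation.
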(event `self.Move`
  ;[1 1 1] Moving event which overwrites Move event in parent blueprint
  (`|AIMoveTo` self (`NavigationSystemV1.K2_GetRandomReachablePointInRadius` (`self.K2_GetActorLocation`) 600.0 null null) null 350.0))

(event `self.Attack`
  (bind _firepoint (`self.FirePoint`))
  ;[1 1 1] Attacking event which overwrites Attack event in parent blueprint
  (`|SpawnActorFromClass` "/Game/StudentWork/Blueprints/EnemiesAndTraps/BP_EnemyProjectile_FastWeak.BP_EnemyProjectile_FastWeak_C" (`KismetMathLibrary.MakeTransform` (`SceneComponent.K2_GetComponentLocation` _firepoint) (`SceneComponent.K2_GetComponentRotation` _firepoint)) "Undefined" "MultiplyWithRoot" null null))

(fn `UserConstructionScript`
  (`parent.UserConstructionScript`))