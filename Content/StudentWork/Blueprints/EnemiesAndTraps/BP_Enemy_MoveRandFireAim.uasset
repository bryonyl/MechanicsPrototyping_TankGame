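; Enemy Blueprint that fires aimed projectiles and counts toward Level 4's kill objective.
; BeginPlay caches actors tagged EnemyTarget and the game instance.
; The overridden parent Attack spawns a fast, weak projectile from FirePoint toward each valid target using look-at rotation.
; After damage, a dead enemy in Level 4 increments the game instance's kill counter, triggering the BP_Goal spawn event once the threshold is reached.
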(event `self.ReceiveBeginPlay`
  (`parent.ReceiveBeginPlay`)
  (bind _outactors (`GameplayStatics.GetAllActorsOfClassWithTag` "/Script/Engine.Actor" "EnemyTarget"))
  (for _array_element _outactors
    (`KismetArrayLibrary.Array_Add` (`self.EnemyTargetArr`) _array_element))
  (bind _asgi_game_instance (cast `/Game/StudentWork/Blueprints/GI_GameInstance` (`GameplayStatics.GetGameInstance`))
    (:`then`
      (set `self.GameInstanceRef` _asgi_game_instance))
    (:`CastFailed`
      (`KismetSystemLibrary.PrintString` "game instance cast failed"))))

(event `self.Attack`
  (bind _returnvalue (`SceneComponent.K2_GetComponentLocation` (`self.FirePoint`)))
  ;[1 1 1] Attacking event which overwrites Attack event in parent blueprint
  (for _array_element (`self.EnemyTargetArr`)
    (`/Engine/EditorBlueprintResources/StandardMacros.IsValid` _array_element
      (:`Is Valid`
        (`|SpawnActorFromClass` "/Game/StudentWork/Blueprints/EnemiesAndTraps/BP_EnemyProjectile_FastWeak.BP_EnemyProjectile_FastWeak_C" (`KismetMathLibrary.MakeTransform` _returnvalue (`KismetMathLibrary.FindLookAtRotation` _returnvalue (`self.K2_GetActorLocation` _array_element))) "Undefined" "MultiplyWithRoot" null null)))))

(event `self.ReceiveAnyDamage`
  (params (Damage :type "Float (single-precision)") (DamageType :type "DamageType Object Reference") (InstigatedBy :type "Controller Object Reference") (DamageCauser :type "Actor Object Reference"))
  (`parent.ReceiveAnyDamage` Damage DamageType InstigatedBy DamageCauser)
  (`self.CheckIfAllEnemiesDead_Level4`))

(event `CheckIfAllEnemiesDead_Level4`
  (bind _gameinstanceref (`self.GameInstanceRef`))
  (if (and (`self.bEnemyDead`) (`self.bInLevel4`))
    (bind _output_get (set `/Game/StudentWork/Blueprints/GI_GameInstance.Level4_EnemiesKilledCounter` (+ (`/Game/StudentWork/Blueprints/GI_GameInstance.Level4_EnemiesKilledCounter` _gameinstanceref) 1) _gameinstanceref))
    (`KismetSystemLibrary.PrintString` (`KismetStringLibrary.Conv_IntToString` _output_get))
    (if (>= _output_get 7)
      (bind _returnvalue (`GameplayStatics.GetActorOfClass` "/Game/Blueprints/MiscBlueprints/BP_Goal.BP_Goal_C"))
      (`/Game/Blueprints/MiscBlueprints/BP_Goal.OnGoalSpawned` _returnvalue)
      (`KismetSystemLibrary.PrintString` "Goal spawned"))))

(fn `UserConstructionScript`
  (`parent.UserConstructionScript`))