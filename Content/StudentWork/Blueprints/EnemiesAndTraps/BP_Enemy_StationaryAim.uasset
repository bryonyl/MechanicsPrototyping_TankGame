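; Stationary enemy that fires fast, weak projectiles from its fire point, aimed at the player's current location.
; Builds on a parent enemy, caching the game instance on BeginPlay and running kill checks after taking damage.
; When dead, it increments game instance counters: five level 2 kills unlock the reward room door, while seven kills flagged as level 4 spawn the goal.
; The level 2 count has no level check.
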(event `self.ReceiveBeginPlay`
  ;[1 1 1] Reference to game instance for later use
  (`parent.ReceiveBeginPlay`)
  (bind _asgi_game_instance (cast `/Game/StudentWork/Blueprints/GI_GameInstance` (`GameplayStatics.GetGameInstance`)))
  (set `self.GameInstanceRef` _asgi_game_instance))

(event `self.Attack`
  (bind _playercharacterref (`self.PlayerCharacterRef`))
  (bind _returnvalue (`SceneComponent.K2_GetComponentLocation` (`self.FirePoint`)))
  ;[1 1 1] Enemy attacks
  (`/Engine/EditorBlueprintResources/StandardMacros.IsValid` _playercharacterref
    (:`Is Valid`
      (`|SpawnActorFromClass` "/Game/StudentWork/Blueprints/EnemiesAndTraps/BP_EnemyProjectile_FastWeak.BP_EnemyProjectile_FastWeak_C" (`KismetMathLibrary.MakeTransform` _returnvalue (`KismetMathLibrary.FindLookAtRotation` _returnvalue (`self.K2_GetActorLocation` _playercharacterref))) "Undefined" "MultiplyWithRoot" null null))))

(event `self.ReceiveAnyDamage`
  (params (Damage :type "Float (single-precision)") (DamageType :type "DamageType Object Reference") (InstigatedBy :type "Controller Object Reference") (DamageCauser :type "Actor Object Reference"))
  ;[1 1 1] Upon being damaged, the enemy checks if all enemies are dead (for level 2 and level 4)
  (`parent.ReceiveAnyDamage` Damage DamageType InstigatedBy DamageCauser)
  (`self.CheckIfAllEnemiesDead_Level2`)
  (`self.CheckIfAllEnemiesDead_Level4`))

(event `CheckIfAllEnemiesDead_Level2`
  (bind _gameinstanceref (`self.GameInstanceRef`))
  ;[1 1 1] Checks if all enemies are dead in order to fulfill the criteria for level 2 completion
  (if (`self.bEnemyDead`)
    (bind _output_get (set `/Game/StudentWork/Blueprints/GI_GameInstance.Level2_EnemiesKilledCounter` (+ (`/Game/StudentWork/Blueprints/GI_GameInstance.Level2_EnemiesKilledCounter` _gameinstanceref) 1) _gameinstanceref))
    (`KismetSystemLibrary.PrintString` (`KismetStringLibrary.Conv_IntToString` _output_get))
    (if (>= _output_get 5)
      (`self.OnLevel2RewardRoomDoorUnlocked`))))

(event `CheckIfAllEnemiesDead_Level4`
  (bind _gameinstanceref (`self.GameInstanceRef`))
  ;[1 1 1] Checks if all enemies are dead in order to fulfill the criteria for level 4 completion
  (if (and (`self.bEnemyDead`) (`self.bInLevel4`))
    (bind _output_get (set `/Game/StudentWork/Blueprints/GI_GameInstance.Level4_EnemiesKilledCounter` (+ (`/Game/StudentWork/Blueprints/GI_GameInstance.Level4_EnemiesKilledCounter` _gameinstanceref) 1) _gameinstanceref))
    (if (>= _output_get 7)
      (bind _returnvalue (`GameplayStatics.GetActorOfClass` "/Game/Blueprints/MiscBlueprints/BP_Goal.BP_Goal_C"))
      (`/Game/Blueprints/MiscBlueprints/BP_Goal.OnGoalSpawned` _returnvalue)
      (`KismetSystemLibrary.PrintString` "Goal spawned"))))

(fn `UserConstructionScript`
  (`parent.UserConstructionScript`))