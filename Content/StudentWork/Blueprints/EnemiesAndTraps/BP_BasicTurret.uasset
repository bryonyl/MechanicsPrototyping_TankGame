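; BP_BasicTurret is a destructible enemy turret that fires projectiles at a fixed interval, with no targeting logic.
; A looping timer started on BeginPlay spawns BP_EnemyProjectile at the Arrow component's location and rotation.
; Incoming damage lowers health and briefly flashes a red overlay material on base and gun, cleared by a timer.
; The turret destroys itself at zero health; an unconnected material-restore chain remains unused.
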(event `self.ReceiveBeginPlay`
  ;[1 1 1] Turret firing projectiles
  (bind _returnvalue (`KismetSystemLibrary.K2_SetTimerDelegate` (delegate `FireProjectile`) 0.5 true))
  (set `self.TurretFireTimer` _returnvalue))

(event `MakeTurretNormal`
  (`MeshComponent.SetOverlayMaterial` (`self.TurretGun`) null)
  (`MeshComponent.SetOverlayMaterial` (`self.TurretBase`) null))

(event `MakeTurretRed`
  (`MeshComponent.SetOverlayMaterial` (`self.TurretBase`) "/Game/StudentWork/Materials/M_DamageOverlay.M_DamageOverlay")
  (`MeshComponent.SetOverlayMaterial` (`self.TurretGun`) "/Game/StudentWork/Materials/M_DamageOverlay.M_DamageOverlay")
  (`KismetSystemLibrary.K2_SetTimerDelegate` (delegate `MakeTurretNormal`) 0.25))

(event `FireProjectile`
  (bind _arrow (`self.Arrow`))
  ;[1 1 1] Turret firing projectiles
  (`|SpawnActorFromClass` "/Game/StudentWork/Blueprints/EnemiesAndTraps/BP_EnemyProjectile.BP_EnemyProjectile_C" (`KismetMathLibrary.MakeTransform` (`SceneComponent.K2_GetComponentLocation` _arrow) (`SceneComponent.K2_GetComponentRotation` _arrow)) "Undefined" "MultiplyWithRoot" null null))

(event `self.ReceiveAnyDamage`
  (params (Damage :type "Float (single-precision)") (DamageType :type "DamageType Object Reference") (InstigatedBy :type "Controller Object Reference") (DamageCauser :type "Actor Object Reference"))
  ;[1 1 1] Enemy takes damage
  (if (not (`self.bEnemyDead`))
    (set `self.EnemyCurrentHealth` (- (`self.EnemyCurrentHealth`) Damage))
    (`self.MakeTurretRed`)
    (if (<= (`self.EnemyCurrentHealth`) 0.0)
      (`self.EnemyDead`))))

(event `EnemyDead`
  ;[1 1 1] Enemy dies
  (set `self.bEnemyDead` true)
  (`self.K2_DestroyActor`))

(fn `UserConstructionScript`)