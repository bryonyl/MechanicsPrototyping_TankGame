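; BP_Lever is a damage-activated puzzle lever that counts toward unlocking the Level 1 reward room door.
; A hit flips the lever, turns its sphere and light blue, and sets collision to ignore so projectiles cannot push it again.
; Activations increment a counter in GI_GameInstance shared by all levers, and reaching three calls the door-unlocked dispatcher.
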(event `self.ReceiveBeginPlay`
  ;[1 1 1] Sets up reference to game instance so that accessing the game instance is easy within this blueprint
  (bind _asgi_game_instance (cast `/Game/StudentWork/Blueprints/GI_GameInstance` (`GameplayStatics.GetGameInstance`)))
  (set `self.GameInstanceRef` _asgi_game_instance))

(event `self.ReceiveAnyDamage`
  (params (Damage :type "Float (single-precision)") (DamageType :type "DamageType Object Reference") (InstigatedBy :type "Controller Object Reference") (DamageCauser :type "Actor Object Reference"))
  ;[1 1 1] Lever is hit; lever physically moves and a check is carried out to see if all levers have been activated
  (`/Engine/EditorBlueprintResources/StandardMacros.FlipFlop`
    (:`A`
      (`SceneComponent.K2_SetRelativeRotation` (`self.Lever`) (struct :`Pitch` -45.0) false false)
      (set `self.bLeverActivated` true)
      (`PrimitiveComponent.SetMaterial` (`self.Sphere`) 0 "/Game/Materials/MI_EmissiveBlue.MI_EmissiveBlue")
      (`LightComponent.SetLightColor` (`self.PointLight`) (struct :`R` 0.073027 :`G` 0.406174 :`B` 0.693 :`A` 1.0) true))
    (:`B`
      (`SceneComponent.K2_SetRelativeRotation` (`self.Lever`) (struct :`Pitch` 45.0) false false)
      (set `self.bLeverActivated` false)))
  (`self.CheckIfAllLeversActivated`))

(event `CheckIfAllLeversActivated`
  (bind _gameinstanceref (`self.GameInstanceRef`))
  (bind _level1_leverhitcounter (`/Game/StudentWork/Blueprints/GI_GameInstance.Level1_LeverHitCounter` _gameinstanceref))
  ;[1 1 1] Check to see if all levers have been activated. If they have, then open the exit door
  (if (`self.bLeverActivated`)
    (`PrimitiveComponent.SetCollisionResponseToAllChannels` (`self.BoxSensor`) "ECR_Ignore")
    (`PrimitiveComponent.SetCollisionResponseToAllChannels` (`self.Lever`) "ECR_Ignore")
    (`PrimitiveComponent.SetCollisionResponseToAllChannels` (`self.Base`) "ECR_Ignore")
    (`PrimitiveComponent.SetCollisionResponseToAllChannels` (`self.Sphere`) "ECR_Ignore") ; Makes the lever no longer collidable with any player projectiles\nso that player can no longer push lever
    (set `/Game/StudentWork/Blueprints/GI_GameInstance.Level1_LeverHitCounter` (+ (`/Game/StudentWork/Blueprints/GI_GameInstance.Level1_LeverHitCounter` (`self.GameInstanceRef`)) 1) _gameinstanceref) ; This variable is in the game instance as I wanted\nit to be a global variable so that all levers would\nshare the same lever hit counter.
    (`KismetSystemLibrary.PrintString` (`KismetStringLibrary.Conv_IntToString` _level1_leverhitcounter))
    (if (>= _level1_leverhitcounter 3)
      (`self.OnLevel1RewardRoomDoorUnlocked`))))

(fn `UserConstructionScript`)