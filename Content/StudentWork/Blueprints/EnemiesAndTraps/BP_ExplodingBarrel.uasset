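; Exploding barrel trap that, the first time it takes any damage, flashes, explodes and unlocks the Maintenance Room 3 door.
; Construction creates a red dynamic flash material, which a timeline animates through its FlashLevel parameter.
; When the timeline finishes, a sphere trace damages hit actors, the barrel destroys itself and spawns a fiery Niagara explosion.
; It then finds the door with GetActorOfClass and calls its unlock event.
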(event `self.ReceiveAnyDamage`
  (params (Damage :type "Float (single-precision)") (DamageType :type "DamageType Object Reference") (InstigatedBy :type "Controller Object Reference") (DamageCauser :type "Actor Object Reference"))
  (bind _returnvalue (`self.K2_GetActorLocation`))
  (`/Engine/EditorBlueprintResources/StandardMacros.DoOnce` false
    (:`Completed`
      (bind (_direction _flash) (`Timeline|Flash` :!via `PlayFromStart`)
        (:`Update`
          (`MaterialInstanceDynamic.SetScalarParameterValue` (`self.FlashMaterial`) "FlashLevel" _flash))
        (:`Finished`
          (bind _outhits (`KismetSystemLibrary.SphereTraceMulti` _returnvalue _returnvalue 200.0 "TraceTypeQuery1"))
          (for _array_element _outhits
            (`GameplayStatics.ApplyDamage` (`.HitActor` (`GameplayStatics.BreakHitResult` _array_element)) 25.0))
          (`self.K2_DestroyActor`)
          (`NiagaraFunctionLibrary.SpawnSystemAtLocation` "/Game/StudentWork/Particles/NS_FieryExplosion.NS_FieryExplosion" (`self.K2_GetActorLocation`))
          (bind _returnvalue_2 (`GameplayStatics.GetActorOfClass` "/Game/StudentWork/Blueprints/Environment/BP_Door_MaintenanceRoom3.BP_Door_MaintenanceRoom3_C"))
          (`/Game/StudentWork/Blueprints/Environment/BP_Door_MaintenanceRoom3.OnMaintenanceRoom3DoorUnlocked` _returnvalue_2))))))

(fn `UserConstructionScript`
  (bind _returnvalue (`PrimitiveComponent.CreateDynamicMaterialInstance` (`self.StaticMesh`) 0 "/Game/StudentWork/Materials/M_ControlledFlash_Red.M_ControlledFlash_Red" "None")) ; Replaces Element 0 Material, which is the main material
  (set `self.FlashMaterial` _returnvalue))