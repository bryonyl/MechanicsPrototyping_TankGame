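; Parent Blueprint for pickup items, which returns its Item value when picked up and creates a quest from per-instance text.
; BeginPlay builds the interact prompt from the item name and caches the player controller.
; PickUpItem starts a briefly delayed self-destroy, then InitialiseQuest feeds the player character's ACQuestSystem.
; The quest popup's delayed fade-out is scheduled on this actor, which is destroyed before that delay ends.
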(event `self.ReceiveBeginPlay`
  ;[1 1 1] Sets up custom interact prompt text
  (set `/Game/StudentWork/Blueprints/AC_Interactable.CustomInteractPromptText` (`|FormatText` "[E] Pick Up {string}" (`self.Item`)) (`self.AC_Interactable`))
  ;[1 1 1] Creates player controller ref for easy access
  (bind _asbp_mech_player_controller (cast `/Game/StudentWork/Blueprints/BP_MechPlayerController` (`GameplayStatics.GetPlayerController` 0)))
  (set `self.PlayerControllerRef` _asbp_mech_player_controller))

(event `DestroyItem`
  ;[1 1 1] Destroys item
  (`KismetSystemLibrary.Delay` 0.1)
  (`self.K2_DestroyActor`))

(event `InitialiseQuest`
  ;[1 1 1] Sets up quest system to display specific quest information from this item instance
  (`self.PlayerCharacterRef`
    (:`then`
      _)
    (:`else`
      (bind _asbp_player_character (cast `/Game/StudentWork/Blueprints/BP_PlayerCharacter` (`GameplayStatics.GetPlayerCharacter` 0)))))
  (bind _ac_questsystem (`/Game/StudentWork/Blueprints/BP_PlayerCharacter.AC_QuestSystem` _asbp_player_character))
  (`/Game/StudentWork/Blueprints/Quests/AC_QuestSystem.CreateQuest` _ac_questsystem (`self.CustomQuestTypeText`) (`self.CustomQuestText`) (`self.CustomTipText`))
  (`KismetSystemLibrary.Delay` 4.0)
  (`/Game/StudentWork/UI/WBP_QuestPopup.FadeOut` (`/Game/StudentWork/Blueprints/Quests/AC_QuestSystem.QuestPopupWidgetRef` _ac_questsystem)))

(fn `PickUpItem`
  (returns (Item :type String))
  (bind _item (`self.Item`))
  (`KismetSystemLibrary.PrintString` (`KismetStringLibrary.Concat_StrStr` _item " picked up"))
  (`self.DestroyItem`)
  (`self.InitialiseQuest`)
  (return _item))

(fn `UserConstructionScript`)