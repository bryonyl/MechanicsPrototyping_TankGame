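; Quest system component that shows a timed popup with a quest's type, description and tip.
; CreateQuest caches the player character, writes the three texts to that character's quest component, then runs the update, display and remove events on itself.
; The events lazily create a WBP_QuestPopup, tell it to refresh its text, add it to the viewport and fade it out after a short delay.
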(event `UpdateText`
  (bind _questpopupwidgetref (`self.QuestPopupWidgetRef`)
    (:`then`
      _)
    (:`else`
      (bind _returnvalue (`|CreateWidget` "/Game/StudentWork/UI/WBP_QuestPopup.WBP_QuestPopup_C"))
      (bind _output_get (set `self.QuestPopupWidgetRef` _returnvalue))))
  (`/Game/StudentWork/UI/WBP_QuestPopup.UpdateQuestTypeText` _output_get)
  (`/Game/StudentWork/UI/WBP_QuestPopup.UpdateQuestTypeText` _questpopupwidgetref)
  (`/Game/StudentWork/UI/WBP_QuestPopup.UpdateQuestText` _output_get)
  (`/Game/StudentWork/UI/WBP_QuestPopup.UpdateQuestText` _questpopupwidgetref)
  (`/Game/StudentWork/UI/WBP_QuestPopup.UpdateTipText` _output_get)
  (`/Game/StudentWork/UI/WBP_QuestPopup.UpdateTipText` _questpopupwidgetref))

(event `DisplayWidget`
  (bind _questpopupwidgetref (`self.QuestPopupWidgetRef`)
    (:`then`
      _)
    (:`else`
      (bind _returnvalue (`|CreateWidget` "/Game/StudentWork/UI/WBP_QuestPopup.WBP_QuestPopup_C"))
      (bind _output_get (set `self.QuestPopupWidgetRef` _returnvalue))))
  (`UserWidget.AddToViewport` _output_get 0)
  (`UserWidget.AddToViewport` _questpopupwidgetref 0))

(event `RemoveWidget`
  (bind _questpopupwidgetref (`self.QuestPopupWidgetRef`)
    (:`then`
      (`KismetSystemLibrary.Delay` 3.0)
      (`/Game/StudentWork/UI/WBP_QuestPopup.FadeOut` _questpopupwidgetref))
    (:`else`)))

(fn `CreateQuest`
  (params (QuestTypeText :type Text) (QuestText :type Text) (QuestTipText :type Text))
  (bind _playercharacterref (`self.PlayerCharacterRef`)
    (:`then`
      _)
    (:`else`
      (bind _asbp_player_character (cast `/Game/StudentWork/Blueprints/BP_PlayerCharacter` (`GameplayStatics.GetPlayerCharacter` 0)))
      (set `self.PlayerCharacterRef` _asbp_player_character)))
  (bind _ac_questsystem (`/Game/StudentWork/Blueprints/BP_PlayerCharacter.AC_QuestSystem` _playercharacterref))
  (set `/Game/StudentWork/Blueprints/Quests/AC_QuestSystem.QuestTypeInfo` QuestTypeText _ac_questsystem)
  (set `/Game/StudentWork/Blueprints/Quests/AC_QuestSystem.QuestInfo` QuestText _ac_questsystem)
  (set `/Game/StudentWork/Blueprints/Quests/AC_QuestSystem.TipInfo` QuestTipText _ac_questsystem)
  (`self.UpdateText`)
  (`self.DisplayWidget`)
  (`self.RemoveWidget`)
  (return))