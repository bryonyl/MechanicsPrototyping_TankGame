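; BP_QuestTriggerBox is a one-shot trigger actor that creates a quest when the player character overlaps it.
; On overlap, InitialiseQuest resolves the player character and calls CreateQuest on its ACQuestSystem component.
; The custom type, quest and tip text on each instance supply the quest information, and the trigger destroys itself afterwards.
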(event `InitialiseQuest`
  ;[1 1 1] Sets up quest system to display specific quest information from this quest trigger box instance
  (`self.PlayerCharacterRef`
    (:`then`
      _)
    (:`else`
      (bind _asbp_player_character (cast `/Game/StudentWork/Blueprints/BP_PlayerCharacter` (`GameplayStatics.GetPlayerCharacter` 0)))))
  (`/Game/StudentWork/Blueprints/Quests/AC_QuestSystem.CreateQuest` (`/Game/StudentWork/Blueprints/BP_PlayerCharacter.AC_QuestSystem` _asbp_player_character) (`self.CustomQuestTypeText`) (`self.CustomQuestText`) (`self.CustomTipText`))
  (`self.K2_DestroyActor`))

(event `self.ReceiveActorBeginOverlap`
  (params (OtherActor :type "Actor Object Reference"))
  (cast `/Game/StudentWork/Blueprints/BP_PlayerCharacter` OtherActor)
  (`self.InitialiseQuest`))

(fn `UserConstructionScript`)